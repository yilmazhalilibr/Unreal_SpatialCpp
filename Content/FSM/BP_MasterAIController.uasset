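; BP_MasterAIController is a base AI controller that starts the BT_MasterShooter behavior tree and stores player pawn 0 in the blackboard on BeginPlay.
; On each successfully sensed perception update, it saves the actor and stimulus, then routes by sense class to Touch, Damage, Hearing, Prediction or Sight functions.
; These five handlers are empty here, and lost-stimulus updates are ignored.
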(event OnTargetPerceptionUpdated(AIPerceptionComponent)
  (params (Actor :type Actor%20Object%20Reference) (Stimulus :type AI%20Stimulus%20Structure))
  (if (Utilities|Struct|BreakAIStimulus Stimulus)
    (Variables|Default|SetStimilusActor Actor)
    (bind _output_get (Variables|Default|SetStimilusData Stimulus))
    (bind _returnvalue (Class|AIPerceptionSystem|GetSenseClassforStimulus _output_get))
    (if (== _returnvalue "/Script/AIModule.AISense_Touch")
      (Utilities|Touch)
      (elif (== _returnvalue "/Script/AIModule.AISense_Damage")
        (Utilities|Damage)
        (elif (== _returnvalue "/Script/AIModule.AISense_Hearing")
          (Utilities|Hearing)
          (elif (== _returnvalue "/Script/AIModule.AISense_Prediction")
            (Utilities|Prediction)
            (elif (== _returnvalue "/Script/AIModule.AISense_Sight")
              (Utilities|Sight))))))))

(event EventBeginPlay
  (|CallParentFunction)
  (AI|RunBehaviorTree "/Game/FSM/BT_MasterShooter.BT_MasterShooter")
  (AI|Components|Blackboard|SetValueasObject (AI|GetBlackboard 0) (Variables|Default|GetPlayerKey) (Game|Player|GetPlayerPawn 0)))

(event EventTick
  (params (DeltaSeconds :type Float%20%28single-precision%29)))

(fn ConstructionScript)