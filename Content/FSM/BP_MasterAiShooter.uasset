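; BP_MasterAiShooter is an AI shooter character driven by a state machine on its MasterAiController.
; OnChangeState alternates the controller between its Patrol and Idle states through a FlipFlop, printing "fail" if the controller cast fails.
; PlayMontageAttack plays the rifle firing montage on the mesh.
; Locomotion setup calls for overlay, stance, rotation mode and a looping sprint gait are present but never run.
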(event Custom|OnChangeState
  (bind _asmaster_ai_controller (Utilities|Casting|CastToMasterAiController (Pawn|GetController))
    (:then
      (Utilities|FlowControl|FlipFlop
        (:A
          (Class|MasterAiController|ChangeStateAI _asmaster_ai_controller (Variables|/Script/Unreal_SpatialCpp.MasterAiController|GetPatrolState _asmaster_ai_controller)))
        (:B
          (Class|MasterAiController|ChangeStateAI _asmaster_ai_controller (Variables|/Script/Unreal_SpatialCpp.MasterAiController|GetIdleState _asmaster_ai_controller)))))
    (:CastFailed
      (Development|PrintString "fail"))))

(event Custom|PlayMontageAttack
  (Animation|Montage|PlayMontage (Variables|Character|GetMesh) "/Game/FSM/FiringRifle_UE_Montage.FiringRifle_UE_Montage"))

(event EventBeginPlay)

(fn ConstructionScript
  (|CallParentFunction))