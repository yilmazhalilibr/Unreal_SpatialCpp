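; BP_Knife is an item Blueprint that defines the Slkrion Knife, a hand-type item for the spatial inventory.
; An override of GetDefaultItemObject constructs an ItemObject from hard-coded item data covering stats, value, grid dimensions, icons and its own class.
; The construction script stores that object in the ItemObject variable, while BeginPlay calls the same function without using the result.
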(event EventBeginPlay
  (CallFunction|GetDefaultItemObjectImplementation))

(fn ConstructionScript
  (bind _returnvalue (CallFunction|GetDefaultItemObjectImplementation))
  (Variables|Default|SetItemObject _returnvalue))

(fn GetDefaultItemObjectImplementation
  (bind _returnvalue (Game|ConstructObjectfromClass self "/Script/Unreal_SpatialCpp.ItemObject" (Utilities|Struct|MakeItemData "Slkrion Knife" "Ordinary Knife" "3.Hand" "None" 5 "(X=0.000000,Y=0.000000)" false 1 95.0 (Utilities|Array|MakeArray (Utilities|Struct|MakeStat "CriticalChange" 25.0)) false "BP_Knife_C" "/Game/SpatialInventory/Icons/M_Icon_Knife.M_Icon_Knife" "/Game/SpatialInventory/Icons/M_Icon_Knife_R.M_Icon_Knife_R" (Utilities|Struct|MakeIntPoint 2 4))))
  (return _returnvalue))