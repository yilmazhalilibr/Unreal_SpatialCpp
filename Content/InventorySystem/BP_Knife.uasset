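; BP_Knife is the knife item in the inventory system, supplying its own inventory data.
; On BeginPlay it keeps a valid ItemObject or creates a default one, printing debug text either way.
; GetDefaultItemObject spawns a BP_ItemObject with the knife's grid size, normal and rotated icons, and BP_Knife as item class.
; The spawn location is the player's scaled forward vector, without adding the pawn's position.
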(event EventBeginPlay
  (|CallParentFunction)
  (Utilities|IsValid (Variables|Default|GetItemObject)
    (:Is%20Valid
      (Development|PrintString "Valid"))
    (:Is%20Not%20Valid
      (bind __itemobject (CallFunction|GetDefaultItemObjectImplementation))
      (bind _output_get (Variables|Default|SetItemObject __itemobject))
      (Development|PrintString (Utilities|GetDisplayName _output_get)))))

(fn ConstructionScript
  (|CallParentFunction))

(fn GetDefaultItemObjectImplementation
  (bind _returnvalue (Game|SpawnActorfromClass "/Game/InventorySystem/BP_ItemObject.BP_ItemObject_C" (Math|Transform|MakeTransform (* (Transformation|GetActorForwardVector (Game|Player|GetPlayerPawn 0)) "11.000000,11.000000,11.000000") "0, 0, 0" "1.000000,1.000000,1.000000") "Undefined" "MultiplyWithRoot" 0 (Utilities|Struct|MakeIntPoint 1 3) "/Game/FPS_Weapon_Bundle/Weapons/Materials/M9_Knife/M_M9_Knife.M_M9_Knife" "/Game/InventorySystem/M_IconBase_Knife_R.M_IconBase_Knife_R" "BP_Knife_C" 0))
  (return _returnvalue))